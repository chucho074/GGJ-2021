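; BP_Monster is a base monster that hurts the player by proximity and can disguise itself as furniture.
; Each Tick applies damage scaled by FearAmount in distance bands; the weakest band repeats the middle band's range, so it never fires.
; Teleport moves it to a random nearby navigable point.
; SwapToFurniture hides Mesh and shows the StaticMesh hidden at BeginPlay; capsule hit damage is unwired.
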(event OnComponentHit(CapsuleComponent)
  (params (HitComponent :type Primitive%20Component%20Object%20Reference) (OtherActor :type Actor%20Object%20Reference) (OtherComp :type Primitive%20Component%20Object%20Reference) (NormalImpulse :type Vector :default "0, 0, 0") (Hit :type Hit%20Result%20Structure%20%28by%20ref%29))
  ;[1 1 1] Comment
)

(event EventBeginPlay
  (Rendering|SetVisibility (Variables|Default|GetStaticMesh) false false))

(event Collision|EventActorBeginOverlap
  (params (OtherActor :type Actor%20Object%20Reference)))

(event EventTick
  (params (DeltaSeconds :type Float%20%28single-precision%29))
  (bind _returnvalue (Transformation|GetActorLocation))
  (bind _player (Variables|Default|GetPlayer))
  (bind _returnvalue_2 (Transformation|GetActorLocation _player))
  (bind _returnvalue_3 (- _returnvalue_2 _returnvalue))
  (bind _returnvalue_4 (Math|Vector|VectorLength _returnvalue_3))
  (Utilities|IsValid _player
    (:Is%20Valid
      (if (Math|Float|InRange(Float) _returnvalue_4 0.0 1.5e+02)
        (Game|Damage|ApplyDamage (Variables|Default|GetPlayer) (* (Variables|Default|GetFearAmount) 1e+01) 0 0)
        (elif (Math|Float|InRange(Float) _returnvalue_4 151.0 3e+02)
          (Game|Damage|ApplyDamage (Variables|Default|GetPlayer) (* (Variables|Default|GetFearAmount) 5.0) 0 0)
          (elif (Math|Float|InRange(Float) _returnvalue_4 151.0 3e+02)
            (Game|Damage|ApplyDamage (Variables|Default|GetPlayer) (* (Variables|Default|GetFearAmount) 2.0) 0 0)))))))

(fn ConstructionScript)

(fn Teleport
  (bind _returnvalue (Transformation|SetActorLocation (.RandomLocation (Class|NavigationSystemV1|GetRandomPointinNavigableRadius (Transformation|GetActorLocation) 1.5e+03 0 0)) false false))
  (return _returnvalue))

(fn SwaptoFurniture
  (Rendering|SetVisibility (Variables|Character|GetMesh) false false)
  (Rendering|SetVisibility (Variables|Default|GetStaticMesh) true false))